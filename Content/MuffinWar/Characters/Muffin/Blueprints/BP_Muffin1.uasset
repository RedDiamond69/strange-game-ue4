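; BP_Muffin1 is an AI-controlled muffin character that kills any BP_Muffin it touches.
; Both actor overlap and Hitbox overlap call OnDeath on the other muffin.
; Its own OnDeath runs once: it disables the Hitbox, stops the AI brain, waits, resets the mesh material, then destroys the actor.
; DoAttack is empty, with its hitbox toggle left disconnected, as are leftover spawn and widget nodes.
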(event `self.ReceiveBeginPlay`)

(event `self.ReceiveActorBeginOverlap`
  (params (OtherActor :type "Actor Object Reference"))
  (bind _asbp_muffin (cast `/Game/MuffinWar/Characters/Muffin/Blueprints/BP_Muffin` OtherActor))
  (`/Game/MuffinWar/Characters/Muffin/Blueprints/BP_Muffin.OnDeath` _asbp_muffin))

(event `self.Hitbox.OnComponentBeginOverlap`
  (params (OverlappedComponent :type "PrimitiveComponent Object Reference") (OtherActor :type "Actor Object Reference") (OtherComp :type "PrimitiveComponent Object Reference") (OtherBodyIndex :type Integer) (bFromSweep :type Boolean) (SweepResult :type "HitResult Structure (by ref)"))
  (`|ExecutionSequence`
    (:`then_0`
      (bind _asbp_muffin (cast `/Game/MuffinWar/Characters/Muffin/Blueprints/BP_Muffin` OtherActor))
      (`/Game/MuffinWar/Characters/Muffin/Blueprints/BP_Muffin.OnDeath` _asbp_muffin))))

(event `OnDeath`
  (if (not (`self.IsDead`))
    (`PrimitiveComponent.SetCollisionEnabled` (`self.Hitbox`) "NoCollision")
    (set `self.IsDead` true)
    (`BrainComponent.StopLogic` (`AIController.BrainComponent` (`AIBlueprintHelperLibrary.GetAIController` self)) "")
    (`KismetSystemLibrary.Delay` 1.5)
    (`PrimitiveComponent.SetMaterial` (`self.Mesh`) 0 null)
    (`KismetSystemLibrary.Delay` 0.2)
    (`self.K2_DestroyActor`)))

(fn `DoAttack`
  (params (IsAttacking :type Boolean)))

(fn `UserConstructionScript`)